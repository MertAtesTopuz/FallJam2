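; BP_PLant is a plant actor, built around a Cube component, that responds to the player character's PlantsAttack event with an explosion effect.
; On BeginPlay it applies its Material variable to the cube and multiplies its Z scale by the NewMesh value.
; It then casts the player to BP_ThirdPersonCharacter and binds its Attack event, which only spawns P_Explosion at the cube's location.
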(event Custom|Attack
  (Effects|SpawnEmitteratLocation "/Game/StarterContent/Particles/P_Explosion.P_Explosion" (Transformation|GetWorldLocation (Variables|Default|GetCube))))

(event EventBeginPlay
  (bind _returnvalue (Transformation|GetActorScale3D))
  (Utilities|FlowControl|Sequence
    (:then_0
      (Rendering|Material|SetMaterial (Variables|Default|GetCube) 0 (Variables|Default|GetMaterial))
      (Transformation|SetActorScale3D (Math|Vector|MakeVector (.x _returnvalue) (.y _returnvalue) (* (.z _returnvalue) (Variables|Default|GetNewMesh)))))
    (:then_1
      (bind _asbp_third_person_character (Utilities|Casting|CastToBP_ThirdPersonCharacter (Game|GetPlayerCharacter 0)))
      (EventDispatchers|BindEventtoPlantsAttack _asbp_third_person_character (delegate Custom|Attack)))))

(fn ConstructionScript)