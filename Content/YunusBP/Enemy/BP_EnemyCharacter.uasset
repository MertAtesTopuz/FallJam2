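; Enemy character that seeks whatever lies ahead of it, using a simple looping behavior started on BeginPlay.
; Every two seconds it line-traces forward from TargetFinder for WorldDynamic objects, with persistent debug drawing, and stores the result as HitTarget, even on a miss.
; It then issues an AI MoveTo toward that actor and plays a jump montage when the move succeeds.
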(event Custom|Walk
  (AI|AIMoveTo self "0, 0, 0" (Variables|Default|GetHitTarget) 4e+01 true
    (:OnSuccess
      (Animation|Montage|PlayMontage (Variables|Character|GetMesh) "/Game/Characters/Mannequins/Animations/Manny/MM_Jump_Montage.MM_Jump_Montage"))))

(event EventBeginPlay
  (CallFunction|LookforTarget :!label _label)
  (CallFunction|Walk)
  (Utilities|FlowControl|Delay 2.0)
  (goto _label))

(fn ConstructionScript)

(fn LookforTarget
  (bind _targetfinder (Variables|Default|GetTargetFinder))
  (bind _returnvalue (Transformation|GetWorldLocation _targetfinder))
  (bind _outhit (Collision|LineTraceForObjects _returnvalue (+ _returnvalue (* (Math|Vector|GetForwardVector _targetfinder) 1e+03)) (Utilities|Array|MakeArray "ObjectTypeQuery2") false 0 "Persistent"))
  (Variables|Default|SetHitTarget (.HitActor (Collision|BreakHitResult _outhit))))