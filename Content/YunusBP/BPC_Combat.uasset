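; BPC_Combat is a combat helper component that handles damage values and the matching animations for attacking and getting hit.
; DealDamage and TakeDamage read a combat struct and trigger events that play its attack or hit montage when that montage is valid.
; DealDamage returns the struct's damage, while TakeDamage returns health minus damage without storing it, leaving the caller to apply the result.
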(event Custom|DealDamageAnim
  (params (Mesh :type Skeletal%20Mesh%20Component%20Object%20Reference) (Anim :type Anim%20Montage%20Object%20Reference))
  (Utilities|IsValid Anim
    (:Is%20Valid
      (Animation|Montage|PlayMontage Mesh Anim))))

(event Custom|TakeDamageAnim
  (params (Mesh :type Skeletal%20Mesh%20Component%20Object%20Reference) (Anim :type Anim%20Montage%20Object%20Reference))
  (Utilities|IsValid Anim
    (:Is%20Valid
      (Animation|Montage|PlayMontage Mesh Anim))))

(fn DealDamage
  (params (S_Combat :type S%20Combat%20Structure))
  (CallFunction|DealDamageAnim (.mesh S_Combat) (.attack S_Combat))
  (return (.damage S_Combat)))

(fn TakeDamage
  (params (S_Combat :type S%20Combat%20Structure))
  (CallFunction|TakeDamageAnim (.mesh S_Combat) (.takedamageanim S_Combat))
  (return (- (.health S_Combat) (.damage S_Combat))))