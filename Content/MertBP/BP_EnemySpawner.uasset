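; BP_EnemySpawner periodically spawns an enemy at one of five spawn point components.
; On BeginPlay it collects the points into an array and starts a looping timer bound to the SpawnEnemy event.
; Each tick of the timer picks a random point and spawns the class held in a variable, using only that point's world location for the transform.
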(event Custom|SpawnEnemy
  (Variables|Default|SetSpawnTransform (Utilities|Array|Get(acopy) (Variables|Default|GetNewVar_0) (Math|Random|RandomIntegerinRange 0 4)))
  (Game|SpawnActorfromClass (Variables|Default|GetNewVar) (Math|Conversions|ToTransform(Vector) (Transformation|GetWorldLocation (Variables|Default|GetSpawnTransform))) "Undefined" "MultiplyWithRoot" 0 0))

(event EventBeginPlay
  (bind _newvar_0 (Variables|Default|GetNewVar_0))
  (Utilities|FlowControl|Sequence
    (:then_0
      (Utilities|Array|Add _newvar_0 (Variables|Default|GetSpawnPoint5))
      (Utilities|Array|Add _newvar_0 (Variables|Default|GetSpawnPoint4))
      (Utilities|Array|Add _newvar_0 (Variables|Default|GetSpawnPoint3))
      (Utilities|Array|Add _newvar_0 (Variables|Default|GetSpawnPoint2))
      (Utilities|Array|Add _newvar_0 (Variables|Default|GetSpawnPoint1)))
    (:then_1
      (Utilities|Time|SetTimerbyEvent (delegate Custom|SpawnEnemy) 3.0 true))))

(fn ConstructionScript)