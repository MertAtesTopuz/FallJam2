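; BP_UltiPnl opens the UltiUI panel and tracks a bar value that the player builds up with key presses.
; Space creates a new UltiUI widget, adds it to the viewport and flags the panel as open, with no check for an existing one.
; While that flag is set, each D or F press raises BarValue by a fixed step, with no clamp or reset.
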(event EventBeginPlay)

(event Input|KeyboardEvents|SpaceBar
  (params (Key :type Key%20Structure :default "None"))
  (:Pressed
    (bind _returnvalue (UserInterface|CreateWidget "/Game/MertBP/UltiUI.UltiUI_C"))
    (UserInterface|Viewport|AddtoViewport _returnvalue 0)
    (Variables|Default|SetisUltiPnlOpen true)))

(event Input|KeyboardEvents|D
  (params (Key :type Key%20Structure :default "None"))
  (:Pressed
    (if (== (Variables|Default|GetisUltiPnlOpen) true)
      (Variables|Default|SetBarValue (+ (Variables|Default|GetBarValue) 0.1)))))

(event Input|KeyboardEvents|F
  (params (Key :type Key%20Structure :default "None"))
  (:Pressed
    (if (== (Variables|Default|GetisUltiPnlOpen) true)
      (Variables|Default|SetBarValue (+ (Variables|Default|GetBarValue) 0.1)))))

(fn ConstructionScript)