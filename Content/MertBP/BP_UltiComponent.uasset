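; Ultimate-charge minigame Blueprint where alternating J and K presses fill a bar within a five-second countdown.
; SpaceBar spawns the UltiUI widget and starts a looping one-second timer that updates the countdown text, closing the panel and resetting the bar at zero.
; Alternating key flags gate each bar increment and highlight the pressed key.
; A full bar removes the panel after a short delay, without clearing the timer or resetting the bar.
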(event Custom|TimerEvent
  ;[0 0 0] SpaceBar
  (Variables|Default|SetTime (- (Variables|Default|GetTime) 1))
  (Variables|/Script/UMG.TextBlock|SetText (Variables|/Game/MertBP/UltiUI.UltiUI_C|GetTimer (Variables|Default|GetUltiUIRef)) (Utilities|Text|ToText(Integer) (Variables|Default|GetTime)))
  (if (<= (Variables|Default|GetTime) 0)
    (Variables|Default|SetisUltiPnlOpen false)
    (Variables|Default|SetBarValue 0.0)
    (Widget|RemovefromParent (Variables|Default|GetUltiUIRef))))

(event EventBeginPlay)

(event EventTick
  (params (DeltaSeconds :type Float%20%28single-precision%29))
  ;[0 0 0] SpaceBar
)

(event Input|KeyboardEvents|SpaceBar
  (params (Key :type Key%20Structure :default "None"))
  ;[0 0 0] SpaceBar
  (:Pressed
    (if (== (Variables|Default|GetisUltiPnlOpen) false)
      (bind _returnvalue (UserInterface|CreateWidget "/Game/MertBP/UltiUI.UltiUI_C"))
      (bind _output_get (Variables|Default|SetUltiUIRef _returnvalue))
      (UserInterface|Viewport|AddtoViewport _output_get 0)
      (Variables|Default|SetisUltiPnlOpen true)
      (Variables|Default|SetTime 5)
      (Variables|/Script/UMG.TextBlock|SetText (Variables|/Game/MertBP/UltiUI.UltiUI_C|GetTimer (Variables|Default|GetUltiUIRef)) (Utilities|Text|ToText(Integer) (Variables|Default|GetTime)))
      (Utilities|Time|SetTimerbyEvent (delegate Custom|TimerEvent) 1.0 true))))

(event Input|KeyboardEvents|J
  (params (Key :type Key%20Structure :default "None"))
  (bind _ultiuiref (Variables|Default|GetUltiUIRef))
  ;[0 0 0] J
  (:Pressed
    (if (== (Variables|Default|GetisUltiPnlOpen) true)
      (if (== (Variables|Default|GetisKPresed) true)
        (Variables|Default|SetisJPresed true)
        (Variables|Default|SetisKPresed false)
        (Appearance|SetColorandOpacity (Variables|/Game/MertBP/UltiUI.UltiUI_C|GetJInput _ultiuiref) "(R=1.000000,G=0.081971,B=0.129741,A=1.000000)" :!class /Script/UMG.Image)
        (Appearance|SetColorandOpacity (Variables|/Game/MertBP/UltiUI.UltiUI_C|GetKInput _ultiuiref) "(R=1.000000,G=1.000000,B=1.000000,A=1.000000)" :!class /Script/UMG.Image)
        (bind _output_get (Variables|Default|SetBarValue (+ (Variables|Default|GetBarValue) 0.02)))
        (Variables|/Script/UMG.ProgressBar|SetPercent (Variables|/Game/MertBP/UltiUI.UltiUI_C|GetUltiBar (Variables|Default|GetUltiUIRef)) _output_get)
        (if (>= (Variables|Default|GetBarValue) 1.0)
          (Variables|Default|SetBarValue 1.0)
          (if (== (Variables|Default|GetBarValue) 1.0)
            (Utilities|FlowControl|Delay 0.2)
            (Variables|Default|SetisUltiPnlOpen false)
            (Widget|RemovefromParent (Variables|Default|GetUltiUIRef))))))))

(event Input|KeyboardEvents|K
  (params (Key :type Key%20Structure :default "None"))
  (bind _ultiuiref (Variables|Default|GetUltiUIRef))
  ;[0 0 0] k
  (:Pressed
    (if (== (Variables|Default|GetisUltiPnlOpen) true)
      (if (== (Variables|Default|GetisJPresed) true)
        (Variables|Default|SetisKPresed true)
        (Variables|Default|SetisJPresed false)
        (Appearance|SetColorandOpacity (Variables|/Game/MertBP/UltiUI.UltiUI_C|GetKInput _ultiuiref) "(R=1.000000,G=0.926995,B=0.000000,A=1.000000)" :!class /Script/UMG.Image)
        (Appearance|SetColorandOpacity (Variables|/Game/MertBP/UltiUI.UltiUI_C|GetJInput _ultiuiref) "(R=1.000000,G=1.000000,B=1.000000,A=1.000000)" :!class /Script/UMG.Image)
        (bind _output_get (Variables|Default|SetBarValue (+ (Variables|Default|GetBarValue) 0.02)))
        (Variables|/Script/UMG.ProgressBar|SetPercent (Variables|/Game/MertBP/UltiUI.UltiUI_C|GetUltiBar (Variables|Default|GetUltiUIRef)) _output_get)
        (if (>= (Variables|Default|GetBarValue) 1.0)
          (Variables|Default|SetBarValue 1.0)
          (if (== (Variables|Default|GetBarValue) 1.0)
            (Utilities|FlowControl|Delay 0.2)
            (Variables|Default|SetisUltiPnlOpen false)
            (Widget|RemovefromParent (Variables|Default|GetUltiUIRef))))))))